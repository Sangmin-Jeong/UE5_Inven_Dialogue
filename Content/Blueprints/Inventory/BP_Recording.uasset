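; Inventory preview actor that pairs a static mesh with a SceneCaptureComponent2D to capture the displayed mesh.
; UpdateStaticMesh takes a struct, validates its mesh, applies it with its material, moves the capture camera and passes position limits to UpdatePosition.
; UpdatePosition only stores the min and max positions, with no use of them in these graphs.
; ResetMesh swaps in the AnimTreeEd_PreviewFloor mesh as a placeholder.
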(event EventBeginPlay)

(event Collision|EventActorBeginOverlap
  (params (OtherActor :type Actor%20Object%20Reference)))

(event EventTick
  (params (DeltaSeconds :type Float%20%28single-precision%29)))

(fn ConstructionScript)

(fn UpdateStaticMesh
  (params (NewMesh :type Item%20Data%20Structure))
  (bind (_type _mesh _materialinstance _itemtexture _id _itemname _quantity _cameraposition _maxposition _minposition) (Utilities|Struct|BreakItemData NewMesh))
  (bind _staticmesh (Variables|Default|GetStaticMesh))
  (Utilities|IsValid _mesh
    (:Is%20Valid
      (Components|StaticMesh|SetStaticMesh _staticmesh _mesh)
      (Rendering|Material|SetMaterial _staticmesh 0 _materialinstance)
      (Transformation|SetRelativeLocation (Variables|Default|GetSceneCaptureComponent2D) _cameraposition false false)
      (CallFunction|UpdatePosition _minposition _maxposition))))

(fn UpdatePosition
  (params (MinPosition :type Float%20%28double-precision%29) (MaxPosition :type Float%20%28double-precision%29))
  (Variables|Default|SetMinPosition MinPosition)
  (Variables|Default|SetMaxPosition MaxPosition))

(fn ResetMesh
  (Components|StaticMesh|SetStaticMesh (Variables|Default|GetStaticMesh) "/Engine/EditorMeshes/AnimTreeEd_PreviewFloor.AnimTreeEd_PreviewFloor"))
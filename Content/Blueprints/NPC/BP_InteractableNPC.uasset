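; Interactable NPC Blueprint that shows dialogue lines one at a time from its dialogue component.
; BeginPlay caches the DialogueComponent reference.
; DisplayDialogues prints the current DialogueList entry with PrintString, then advances the component's index, wrapping to the first line after the last.
; Nothing in this graph calls DisplayDialogues, and Tick and overlap events are unused.
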(event EventBeginPlay
  (Variables|Default|SetDialogueComp (Variables|Default|GetDialogueComponent)))

(event Collision|EventActorBeginOverlap
  (params (OtherActor :type Actor%20Object%20Reference)))

(event EventTick
  (params (DeltaSeconds :type Float%20%28single-precision%29)))

(fn ConstructionScript)

(fn DisplayDialogues
  (bind _dialoguecomp (Variables|Default|GetDialogueComp))
  (bind _dialoguecomp_2 (Variables|Default|GetDialogueComp))
  (bind _dialoguelist (Variables|/Script/UE5_Inven_Dialogue.DialogueComponent|GetDialogueList _dialoguecomp))
  (Development|PrintString (Utilities|Array|Get(acopy) _dialoguelist (Variables|/Script/UE5_Inven_Dialogue.DialogueComponent|GetCurrentDialogueIndex _dialoguecomp)))
  (bind _result (Math|Integer|IncrementInt (Variables|/Script/UE5_Inven_Dialogue.DialogueComponent|GetCurrentDialogueIndex _dialoguecomp))
    (:%20%20
      (if (>= _result (Utilities|Array|Length _dialoguelist))
        (Variables|/Script/UE5_Inven_Dialogue.DialogueComponent|SetCurrentDialogueIndex _dialoguecomp_2 0)
        (else
          (Variables|/Script/UE5_Inven_Dialogue.DialogueComponent|SetCurrentDialogueIndex _dialoguecomp_2 _result))))))